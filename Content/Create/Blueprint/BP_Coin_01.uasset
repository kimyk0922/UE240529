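; BP_Coin_01 is a coin pickup that responds when a BP_Third_Edit actor overlaps its Coin component.
; The overlap calls EvtPoint on that actor and plays the Coin_Evt_Move timeline, which raises the coin along relative Z.
; A half-second Delay hanging off the timeline update then destroys the coin.
; The yaw-spin timeline and a delayed mesh swap are present but never run.
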(event `self.Coin.OnComponentBeginOverlap`
  (params (OverlappedComponent :type "PrimitiveComponent Object Reference") (OtherActor :type "Actor Object Reference") (OtherComp :type "PrimitiveComponent Object Reference") (OtherBodyIndex :type Integer) (bFromSweep :type Boolean) (SweepResult :type "HitResult Structure (by ref)"))
  (bind _asbp_third_edit (cast `/Game/Create/Blueprint/BP_Third_Edit` OtherActor))
  (`/Game/Create/Blueprint/BP_Third_Edit.Evt_Point` _asbp_third_edit)
  (bind (_direction _newtrack_0) (`Timeline|Coin_Evt_Move`)
    (:`Update`
      (`SceneComponent.K2_SetRelativeLocation` (`self.Coin`) (`KismetMathLibrary.MakeVector` 0.0 0.0 (`KismetMathLibrary.Lerp` 0.0 350.0 _newtrack_0)) false false)
      (`KismetSystemLibrary.Delay` 0.5)
      (`self.K2_DestroyActor`))))

(fn `UserConstructionScript`)
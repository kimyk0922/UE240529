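; BP_Point is a coin pickup that awards a point to the BP_Third_Edit character on overlap.
; The Coin's begin-overlap passes through a DoOnce, casts the other actor, calls its EvtPoint and destroys the pickup.
; A short delay and mesh clear are wired after the destroy call.
; An Animation timeline is set up to spin the coin, but nothing starts it.
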(event `self.Coin.OnComponentBeginOverlap`
  (params (OverlappedComponent :type "PrimitiveComponent Object Reference") (OtherActor :type "Actor Object Reference") (OtherComp :type "PrimitiveComponent Object Reference") (OtherBodyIndex :type Integer) (bFromSweep :type Boolean) (SweepResult :type "HitResult Structure (by ref)"))
  ;[1 1 1 1 12] Once_Overlap_
  (`/Engine/EditorBlueprintResources/StandardMacros.DoOnce` false
    (:`Completed`
      (bind _asbp_third_edit (cast `/Game/Create/Blueprint/BP_Third_Edit` OtherActor))
      (`/Game/Create/Blueprint/BP_Third_Edit.Evt_Point` _asbp_third_edit)
      (`self.K2_DestroyActor`)
      (`KismetSystemLibrary.Delay` 0.2)
      (`StaticMeshComponent.SetStaticMesh` (`self.Coin`) null))))

(fn `UserConstructionScript`)
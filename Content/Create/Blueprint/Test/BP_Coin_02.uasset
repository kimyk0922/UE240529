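; BP_Coin_02 is a test coin pickup that reacts when a BP_Third_Edit_00 actor overlaps it.
; The overlap reassigns that character's Count to itself without incrementing it, then refreshes its TEXT with the value.
; The Point_Movements timeline raises the coin along Z, and the actor destroys itself after a short delay.
; A Coin_Movements timeline for yaw spin exists but is never run.
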(event `self.Coin.OnComponentBeginOverlap`
  (params (OverlappedComponent :type "PrimitiveComponent Object Reference") (OtherActor :type "Actor Object Reference") (OtherComp :type "PrimitiveComponent Object Reference") (OtherBodyIndex :type Integer) (bFromSweep :type Boolean) (SweepResult :type "HitResult Structure (by ref)"))
  (bind _asbp_third_edit_00 (cast `/Game/Create/Blueprint/Test/BP_Third_Edit_00` OtherActor))
  (bind _output_get (set `/Game/Create/Blueprint/Test/BP_Third_Edit_00.Count` (`/Game/Create/Blueprint/Test/BP_Third_Edit_00.Count` _asbp_third_edit_00) _asbp_third_edit_00))
  (`TextRenderComponent.K2_SetText` (`/Game/Create/Blueprint/Test/BP_Third_Edit_00.TEXT` _asbp_third_edit_00) (`KismetTextLibrary.Conv_IntToText` _output_get))
  (bind (_direction _newtrack_0) (`Timeline|Point_Movements`)
    (:`Update`
      (`SceneComponent.K2_SetRelativeLocation` (`self.Coin`) (`KismetMathLibrary.MakeVector` 0.0 0.0 (`KismetMathLibrary.Lerp` 45.0 350.0 _newtrack_0)) false false))
    (:`Finished`
      (`KismetSystemLibrary.Delay` 1.0)
      (`self.K2_DestroyActor`))))

(fn `UserConstructionScript`)
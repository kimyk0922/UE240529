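; BP_Ele is an elevator actor whose Cube moves between its base position and EleValue when a button event fires.
; Box overlap events toggle the OnOff flag, so Evt_Ele_Button only acts while something is inside the Box.
; A FlipFlop alternates playing and reversing Ele_TimeLine, whose track drives a vector lerp of the Cube's relative location without sweep.
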(event `Evt_Ele_Button`
  (if (`self.On/Off`)
    (`/Engine/EditorBlueprintResources/StandardMacros.FlipFlop`
      (:`A`
        (bind (_direction _newtrack_0) (`Timeline|Ele_TimeLine` :!label _label)
          (:`Update`
            (`SceneComponent.K2_SetRelativeLocation` (`self.Cube`) (`KismetMathLibrary.VLerp` (0.0 0.0 0.0) (`self.Ele_Value`) _newtrack_0) false false))))
      (:`B`
        (goto _label :!via `Reverse`)))))

(event `self.Box.OnComponentBeginOverlap`
  (params (OverlappedComponent :type "PrimitiveComponent Object Reference") (OtherActor :type "Actor Object Reference") (OtherComp :type "PrimitiveComponent Object Reference") (OtherBodyIndex :type Integer) (bFromSweep :type Boolean) (SweepResult :type "HitResult Structure (by ref)"))
  (set `self.On/Off` true))

(event `self.Box.OnComponentEndOverlap`
  (params (OverlappedComponent :type "PrimitiveComponent Object Reference") (OtherActor :type "Actor Object Reference") (OtherComp :type "PrimitiveComponent Object Reference") (OtherBodyIndex :type Integer))
  (set `self.On/Off` false))

(fn `UserConstructionScript`)